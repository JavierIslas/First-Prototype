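; Test game mode that awards score for bot kills and spawns enemy bots.
; An actor-killed handler adds points to the killer's SPlayerState when an SCharacter kills a non-player pawn, then prints the score.
; SpawnNewBot runs an EQS query for spawn locations, picking randomly from the best 25%.
; Each returned location gets a debug sphere and a random Enemy_Base_BP or TrackerBot_BP, skipped if collision cannot be resolved.
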(event Custom|OnQueryFinishedEvent_Event_0
  (params (QueryInstance :type Env%20Query%20Instance%20Blueprint%20Wrapper%20Object%20Reference) (QueryStatus :type EEnvQueryStatus%20Enum :default "Processing"))
  (switch Utilities|FlowControl|Switch|SwitchonEEnvQueryStatus QueryStatus
    (:Success
      (for _array_element (Class|EnvQueryInstanceBlueprintWrapper|GetResultsasLocations QueryInstance)
        (Rendering|Debug|DrawDebugSphere _array_element 5e+01 12 "(R=1.000000,G=0.759549,B=0.000000,A=1.000000)" 2.0 2.0)
        (Game|SpawnActorfromClass (select (Math|Random|RandomBool) "/Game/HumanoidEnemy/Enemy_Base_BP.Enemy_Base_BP_C" "/Game/BluePrints/TrackerBot_BP.TrackerBot_BP_C") (Math|Transform|MakeTransform _array_element) "AdjustIfPossibleButDontSpawnIfColliding" 0 0)))))

(event Custom|OnActorKilled_Event_0
  (params (VictimeActor :type Actor%20Object%20Reference) (KillerActor :type Actor%20Object%20Reference) (KillerController :type Controller%20Object%20Reference))
  (bind _returnvalue (Pawn|GetControlledPawn KillerController))
  (bind _playerstate (Variables|/Script/Engine.Pawn|GetPlayerState _returnvalue))
  (Utilities|Casting|CastToSCharacter KillerActor)
  (bind _aspawn (Utilities|Casting|CastToPawn VictimeActor))
  (if (not (Pawn|IsPlayerControlled _aspawn))
    (bind _assplayer_state (Utilities|Casting|CastToSPlayerState _playerstate))
    (Class|SPlayerState|AddScore _assplayer_state 1e+01)
    (Development|PrintString (Utilities|String|ToString(Float) (Variables|/Script/Engine.PlayerState|GetScore _playerstate)))))

(event EventBeginPlay
  (EventDispatchers|AssignOnActorKilled (delegate Custom|OnActorKilled_Event_0)))

(event EventSpawnNewBot
  (bind _returnvalue (AI|EQS|RunEQSQuery "/Game/BluePrints/EQS_FindSpawnLocarion.EQS_FindSpawnLocarion" self "RandomBest25Pct"))
  (EventDispatchers|AssignOnQueryFinishedEvent _returnvalue (delegate Custom|OnQueryFinishedEvent_Event_0)))

(fn ConstructionScript)